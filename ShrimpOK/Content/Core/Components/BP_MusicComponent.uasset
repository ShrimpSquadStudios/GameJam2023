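; BP_MusicComponent is a music component that plays the Gravitation song and steps through its timed note chart.
; On BeginPlay, after a short delay, it loads DT_Gravitation rows into a Notes array, broadcasts OnSongStarted and starts the sound.
; PlayCurrentNote re-triggers itself through Delays based on the gaps between note timestamps.
; Each note currently only prints its index and position as debug text.
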(event `self.ReceiveBeginPlay`
  (`parent.ReceiveBeginPlay`)
  (`KismetSystemLibrary.Delay` 2.0)
  (`KismetSystemLibrary.PrintString` "Game will start in 20 seconds!")
  (bind _outrownames (`DataTableFunctionLibrary.GetDataTableRowNames` "/Game/Data/Songs/DT_Gravitation.DT_Gravitation"))
  (for _array_element _outrownames
    (bind _returnvalue (`|GetDataTableRow` "/Game/Data/Songs/DT_Gravitation.DT_Gravitation" _array_element)
      (:`then`
        (`KismetArrayLibrary.Array_Add` (`self.Notes`) _returnvalue))))
  (`self.OnSongStarted`)
  (`GameplayStatics.PlaySound2D` "/Game/Audio/Gravitation.Gravitation" 1.0 1.0 0.0 null null)
  (bind _output_get (set `self.CurrentNoteIndex` 0))
  (bind _output (`|GetArrayItem` (`self.Notes`) _output_get))
  (set `self.CurrentNote` _output)
  (`KismetSystemLibrary.Delay` (`.Timestamp` (break `MidiNoteRow` _output)))
  (`self.PlayCurrentNote`))

(event `PlayCurrentNote`
  (bind (_currentnote_timestamp _currentnote_position) (break `MidiNoteRow` (`self.CurrentNote`)))
  (bind _currentnoteindex (`self.CurrentNoteIndex`))
  (bind _notes (`self.Notes`))
  (bind _output_timestamp (break `MidiNoteRow` (`|GetArrayItem` _notes _currentnoteindex)))
  (`KismetSystemLibrary.PrintString` (`KismetStringLibrary.Concat_StrStr` (`KismetStringLibrary.Conv_IntToString` (`self.CurrentNoteIndex`)) " " (`|GetEnumeratorNameAsString` _currentnote_position)))
  (bind _result (`/Engine/EditorBlueprintResources/StandardMacros.IncrementInt` (`self.CurrentNoteIndex`))
    (:`  `
      (if (`KismetArrayLibrary.Array_IsValidIndex` _notes _result)
        (`KismetSystemLibrary.Delay` (- _output_timestamp _currentnote_timestamp))
        (set `self.CurrentNote` (`|GetArrayItem` (`self.Notes`) _currentnoteindex))
        (`self.PlayCurrentNote`)))))